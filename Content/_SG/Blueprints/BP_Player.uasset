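; Player character for a top-down 2D game that moves with Enhanced Input and automatically fires fireballs toward the mouse cursor.
; After a short BeginPlay delay it registers itself with the game instance and starts a looping timer that requests pooled bullets from the level manager.
; Movement is blocked when dead, and paired gates choose between horizontal and vertical flipbooks from an animation map, with directional idles on release.
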(event EventBeginPlay
  (Initialization|PreInitialization)
  (Utilities|FlowControl|Delay 0.2)
  (Initialization|PostInitialization))

(fn ConstructionScript)

(fn GetProperAnim
  (params (Str :type String))
  (return (.Value (Utilities|Map|Find (Variables|Presets|GetCharacterAnimations) Str))))

(fn PreInitialization
  (bind _aspc_in_game (Utilities|Casting|CastToPC_InGame (Pawn|GetController)))
  (Utilities|IsValid (PlayerController|LocalPlayerSubsystems|GetEnhancedInputLocalPlayerSubsystem _aspc_in_game)
    (:Is%20Valid
      (Input|AddMappingContext (PlayerController|LocalPlayerSubsystems|GetEnhancedInputLocalPlayerSubsystem _aspc_in_game) "/Game/_SG/Inputs/IMC_SG.IMC_SG" 0 "(bIgnoreAllPressedKeysUntilRelease=True,bForceImmediately=False,bNotifyUserSettings=False)")
      (CallFunction|InitializeCharacterAnim))))

(fn StartPriestFirewand
  (bind _returnvalue (Transformation|GetActorLocation))
  (Default|PoolingBullets (Variables|/Game/_SG/Data/GI_SG.GI_SG_C|GetRef_LevelManager (CallFunction|FlibGetGI)) (Math|Vector|MakeVector (.x _returnvalue) (.y _returnvalue) (- (.z _returnvalue) 2.0)) "1.000000,1.000000,1.000000" 1.0 (* (Math|Rotator|GetRotationXVector (Math|Rotator|MakeRotator 0.0 0.0 (.yaw (Math|Rotator|FindLookatRotation (Transformation|GetActorLocation) (.WorldLocation (Game|Player|ConvertMouseLocationToWorldSpace (Game|GetPlayerController 0))))))) (Variables|Default|GetAtkVel)) "enemy" self "/Game/_SG/Assets/Bullets/FB_FireBall.FB_FireBall" "1.000000,1.000000,1.000000" 3.0))

(fn PostInitialization
  (Variables|/Game/_SG/Data/GI_SG.GI_SG_C|SetRef_Player (CallFunction|FlibGetGI) self)
  (Utilities|Time|SetTimerbyFunctionName 0 "start_priest_firewand" 0.7 true))

(event Custom|InitializeCharacterAnim
  ;[0 0 0] Movement
  (Variables|Runtime|SetMoveState "NewEnumerator1")
  (Sprite|SetFlipbook (Variables|Default|GetPaperFlipbook) (Utilities|Select :Index (Variables|Runtime|GetMoveState) :NewEnumerator0 (Tools|GetProperAnim "idle_up") :NewEnumerator1 (Tools|GetProperAnim "idle_down") :NewEnumerator2 (Tools|GetProperAnim "idle_left") :NewEnumerator3 (Tools|GetProperAnim "idle_right"))))

(event Input|EnhancedActionEvents|EnhancedInputActionIA_Movement
  (params (ActionValue :type Vector%202D%20Structure) (ElapsedSeconds :type Float%20%28double-precision%29) (TriggeredSeconds :type Float%20%28double-precision%29) (InputAction :type Input%20Action%20Object%20Reference :default "/Game/_SG/Inputs/IA_Movement.IA_Movement"))
  (bind (_x _y) (Math|Vector2D|BreakVector2D ActionValue))
  ;[0 0 0] Movement
  (:Triggered
    (Utilities|GeneralCheck
      (:true
        (Variables|Runtime|SetActionValX _x)
        (Variables|Runtime|SetActionValY _y)
        (Pawn|Input|AddMovementInput "1.000000,0.000000,0.000000" (Variables|Runtime|GetActionValX) false) ; Horizontal direction
        (Pawn|Input|AddMovementInput "0.000000,1.000000,0.000000" (Variables|Runtime|GetActionValY) false) ; Vertical Direction
        (Utilities|FlowControl|Sequence
          (:then_0
            (if (!= (Variables|Runtime|GetActionValY) 0.0)
              (Variables|Runtime|SetMoveState (select (> (Variables|Runtime|GetActionValY) 0.0) "NewEnumerator1" "NewEnumerator0"))
              (Utilities|FlowControl|Gate true :!label _label
                (:Exit
                  (Sprite|SetFlipbook (Variables|Default|GetPaperFlipbook) (select (> (Variables|Runtime|GetActionValY) 0.0) (Tools|GetProperAnim "move_down") (Tools|GetProperAnim "move_up")))
                  (goto _label_2 Close)))
              (else
                (goto _label_2 Open))))
          (:then_1
            (if (!= (Variables|Runtime|GetActionValX) 0.0)
              (Variables|Runtime|SetMoveState (select (> (Variables|Runtime|GetActionValX) 0.0) "NewEnumerator3" "NewEnumerator2"))
              (Utilities|FlowControl|Gate true :!label _label_2
                (:Exit
                  (Sprite|SetFlipbook (Variables|Default|GetPaperFlipbook) (select (> (Variables|Runtime|GetActionValX) 0.0) (Tools|GetProperAnim "move_right") (Tools|GetProperAnim "move_left")))
                  (goto _label Close)))
              (else
                (goto _label Open))))))))
  (:Completed
    (Sprite|SetFlipbook (Variables|Default|GetPaperFlipbook) (Utilities|Select :Index (Variables|Runtime|GetMoveState) :NewEnumerator0 (Tools|GetProperAnim "idle_up") :NewEnumerator1 (Tools|GetProperAnim "idle_down") :NewEnumerator2 (Tools|GetProperAnim "idle_left") :NewEnumerator3 (Tools|GetProperAnim "idle_right")))))